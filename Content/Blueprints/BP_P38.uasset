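; BP_P38 is a player-controlled P-38 aircraft pawn that flies forward continuously and fires rockets.
; Tick feeds the forward vector and ForwardSpeed into movement input, with the Slow action lowering the speed while held.
; Pitch and Roll axes add local rotation; only roll is scaled by delta time and RotateSpeed, while pitch uses the raw axis value.
; Fire spawns BP_Rocket at a socket on SMBody.
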(event EventBeginPlay)

(event Collision|EventActorBeginOverlap
  (params (OtherActor :type Actor%20Object%20Reference)))

(event EventTick
  (params (DeltaSeconds :type Float%20%28single-precision%29))
  (Pawn|Input|AddMovementInput (Transformation|GetActorForwardVector) (Variables|Default|GetForward%20Speed) false))

(event Input|ActionEvents|InputActionSlow
  (params (Key :type Key%20Structure :default "None"))
  (:Pressed
    (Variables|Default|SetForward%20Speed 0.3))
  (:Released
    (Variables|Default|SetForward%20Speed 1.0)))

(event Input|ActionEvents|InputActionFire
  (params (Key :type Key%20Structure :default "None"))
  (:Pressed
    (Game|SpawnActorfromClass "/Game/Blueprints/BP_Rocket.BP_Rocket_C" (Transformation|GetSocketTransform (Variables|Default|GetSM_Body) "RocketSpwanPoint" "RTS_World") "Undefined" "MultiplyWithRoot" 0 0)))

(event Input|AxisEvents|InputAxisRoll
  (params (AxisValue :type Float%20%28single-precision%29))
  (Transformation|AddActorLocalRotation (Math|Rotator|MakeRotator (* AxisValue (Utilities|Time|GetWorldDeltaSeconds) (Variables|Default|GetRotate%20Speed)) 0.0 0.0) false false))

(event Input|AxisEvents|InputAxisPitch
  (params (AxisValue :type Float%20%28single-precision%29))
  (Transformation|AddActorLocalRotation (Math|Rotator|MakeRotator 0.0 AxisValue 0.0) false false))

(fn ConstructionScript)